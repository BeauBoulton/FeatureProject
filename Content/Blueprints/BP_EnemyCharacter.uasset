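; BP_EnemyCharacter is an enemy character that reacts to being pushed by a player.
; It caches its ABP_Enemy animation instance at BeginPlay to drive push reactions.
; OnPushed adds an impulse along the pusher's forward vector, scaled by PushStrength.
; A push at the hardcoded full-charge strength turns the enemy toward the player and triggers a fall; others trigger a stagger, and PushEnd follows a short delay.
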(event `self.ReceiveBeginPlay`
  ;[0 0 0 0.5] Get and save a reference to animation blueprint
  (bind _asabp_enemy (cast `/Game/Blueprints/AnimationBlueprints/ABP_Enemy` (`SkeletalMeshComponent.GetAnimInstance` (`self.Mesh`))))
  (set `self.EnemyAnimRef` _asabp_enemy))

(event `/Game/Blueprints/Interfaces/BPI_Pushable.OnPushed`
  (params (InteractingPlayer :type "/Game/Blueprints/Player/BP_PlayerCharacter Object Reference"))
  (bind (_returnvalue_roll _returnvalue_pitch) (`KismetMathLibrary.BreakRotator` (`self.K2_GetActorRotation`)))
  (bind _interacting_player (`self.Interacting Player`))
  (bind _pushstrength (`/Game/Blueprints/Player/BP_PlayerCharacter.PushStrength` _interacting_player))
  (bind (_returnvalue_roll_2 _returnvalue_pitch_2 _returnvalue_yaw) (`KismetMathLibrary.BreakRotator` (`KismetMathLibrary.FindLookAtRotation` (`self.K2_GetActorLocation`) (`self.K2_GetActorLocation` (`self.Interacting Player`)))))
  ;[0 0 0 0.5] Add impulse and play correct animations when pushed
  (set `self.Interacting Player` InteractingPlayer)
  (`CharacterMovementComponent.AddImpulse` (`self.CharacterMovement`) (* (`self.GetActorForwardVector` _interacting_player) _pushstrength) false)
  (if (== _pushstrength 250000.0)
    ;;[0 0 0 0.5] If push is fully charged, rotate to face player and play falling down animation
    (`self.K2_SetActorRotation` (`KismetMathLibrary.MakeRotator` _returnvalue_roll _returnvalue_pitch _returnvalue_yaw))
    (`/Game/Blueprints/AnimationBlueprints/ABP_Enemy.IsFullPushed` (`self.EnemyAnimRef`))
    (else
      ;;[0 0 0 0.5] If push is not fully charged, play stagger animation
      (`/Game/Blueprints/AnimationBlueprints/ABP_Enemy.IsPushed` (`self.EnemyAnimRef`))))
  (`KismetSystemLibrary.Delay` 0.2)
  (`/Game/Blueprints/AnimationBlueprints/ABP_Enemy.PushEnd` (`self.EnemyAnimRef`)))

(fn `UserConstructionScript`)