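; BP_Door is a double door that swings open in response to a player's push.
; OnPushed checks the interacting player's PushStrength while the door is not yet Open.
; A fully charged push plays a timeline that moves and rotates both leaves fully open, setting Open to block further pushes.
; Any other strength plays a second timeline that only rotates the leaves slightly, leaving the door pushable.
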(event `/Game/Blueprints/Interfaces/BPI_Pushable.OnPushed`
  (params (InteractingPlayer :type "/Game/Blueprints/Player/BP_PlayerCharacter Object Reference"))
  (bind _doorr (`self.DoorR`))
  (bind _doorl (`self.DoorL`))
  (bind _alpha (`self.Alpha`))
  (bind _alpha_2 (`self.Alpha`))
  (bind (_returnvalue_location _returnvalue_rotation _returnvalue_scale) (`KismetMathLibrary.BreakTransform` (`SceneComponent.GetRelativeTransform` _doorr)))
  (bind (_returnvalue_location_2 _returnvalue_rotation_2 _returnvalue_scale_2) (`KismetMathLibrary.BreakTransform` (`SceneComponent.GetRelativeTransform` _doorl)))
  ;[0 0 0 0.5] When OnPushed, open doors slightly if push is not fully charged, or fully if fully charged
  ;;[0 0 0 0.5] Checks if doors are not already open and if the push is strong enough to fully open them
  (if (not (`self.Open`))
    (if (== (`/Game/Blueprints/Player/BP_PlayerCharacter.PushStrength` InteractingPlayer) 250000.0)
      ;;[0 0 0 0.5] If push is fully charged, move doors completely open and set Open bool so that doors cannot be pushed again
      (bind (_direction _alpha_3) (`Timeline|Timeline`)
        (:`Update`
          (set `self.Alpha` _alpha_3)
          (`SceneComponent.K2_SetRelativeTransform` _doorr (`KismetMathLibrary.MakeTransform` (`KismetMathLibrary.MakeVector` 210.0 (* _alpha -100.0)) (`KismetMathLibrary.MakeRotator` 0.0 0.0 (* _alpha 90.0)) _returnvalue_scale) false false)
          (`SceneComponent.K2_SetRelativeTransform` _doorl (`KismetMathLibrary.MakeTransform` (`KismetMathLibrary.MakeVector` -210.0 (* _alpha_2 -100.0)) (`KismetMathLibrary.MakeRotator` 0.0 0.0 (* _alpha_2 -90.0)) _returnvalue_scale_2) false false)
          (set `self.Open` true)))
      (else
        ;;[0 0 0 0.5] If push is not strong enough, rotate them open slightly
        (bind (_direction_2 _alpha_4) (`Timeline|Timeline_0`)
          (:`Update`
            (set `self.Alpha_0` _alpha_4)
            (`SceneComponent.K2_SetRelativeRotation` (`self.DoorR`) (`KismetMathLibrary.MakeRotator` 0.0 0.0 (* (`self.Alpha_0`) 10.0)) false false)
            (`SceneComponent.K2_SetRelativeRotation` (`self.DoorL`) (`KismetMathLibrary.MakeRotator` 0.0 0.0 (* (`self.Alpha_0`) -10.0)) false false)))))))

(fn `UserConstructionScript`)