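; Player character with Enhanced Input movement, look and jump, plus a force push ability that acts on pushable actors.
; BeginPlay adds the mapping context, and movement follows control rotation while CanMove is true.
; Force push stops movement, plays a montage and, after a short delay, sphere-traces forward from the capsule over PushRange.
; Hit actors implementing BPI_Pushable receive OnPushed through an interface message.
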(event `self.ReceiveBeginPlay`
  (bind _asbp_player_controller (cast `/Game/Blueprints/Player/BP_PlayerController` (`self.GetController`)))
  (bind _output_get (set `self.PlayerController` _asbp_player_controller))
  (bind _returnvalue (pcsubsystem `EnhancedInputLocalPlayerSubsystem` _output_get))
  (`/Engine/EditorBlueprintResources/StandardMacros.IsValid` _returnvalue
    (:`Is Valid`
      (`EnhancedInputSubsystemInterface.AddMappingContext` _returnvalue "/Game/Inputs/IMC_PlayerControls.IMC_PlayerControls" 0 (struct)))))

(event `EnhancedInput|/Game/Inputs/Actions/IA_Move`
  (params (ActionValue :type "Vector2D Structure") (ElapsedSeconds :type "Float (double-precision)") (TriggeredSeconds :type "Float (double-precision)") (InputAction :type "InputAction Object Reference" :default "/Game/Inputs/Actions/IA_Move.IA_Move"))
  (bind (_returnvalue_x _returnvalue_y) (`KismetMathLibrary.BreakVector` (`KismetMathLibrary.Normal` (`KismetMathLibrary.MakeVector` ActionValue_X ActionValue_Y))))
  (bind (_returnvalue_roll _returnvalue_pitch _returnvalue_yaw) (`KismetMathLibrary.BreakRotator` (`Controller.GetControlRotation` (`self.PlayerController`))))
  (bind (_returnvalue_roll_2 _returnvalue_pitch_2 _returnvalue_yaw_2) (`KismetMathLibrary.BreakRotator` (`Controller.GetControlRotation` (`self.PlayerController`))))
  (:`Triggered`
    (if (`self.CanMove`)
      (`self.AddMovementInput` (`KismetMathLibrary.GetRightVector` (`KismetMathLibrary.MakeRotator` _returnvalue_roll_2 0.0 _returnvalue_yaw_2)) _returnvalue_x)
      (`self.AddMovementInput` (`KismetMathLibrary.GetForwardVector` (`KismetMathLibrary.MakeRotator` 0.0 0.0 _returnvalue_yaw)) _returnvalue_y))))

(event `EnhancedInput|/Game/Inputs/Actions/IA_Look`
  (params (ActionValue :type "Vector2D Structure") (ElapsedSeconds :type "Float (double-precision)") (TriggeredSeconds :type "Float (double-precision)") (InputAction :type "InputAction Object Reference" :default "/Game/Inputs/Actions/IA_Look.IA_Look"))
  (:`Triggered`
    (`self.AddControllerYawInput` ActionValue_X)
    (`self.AddControllerPitchInput` ActionValue_Y)))

(event `EnhancedInput|/Game/Inputs/Actions/IA_Jump`
  (params (ActionValue :type Boolean) (ElapsedSeconds :type "Float (double-precision)") (TriggeredSeconds :type "Float (double-precision)") (InputAction :type "InputAction Object Reference" :default "/Game/Inputs/Actions/IA_Jump.IA_Jump"))
  (:`Started`
    (`self.Jump`))
  (:`Canceled`
    (`self.StopJumping`)))

(event `EnhancedInput|/Game/Inputs/Actions/IA_ForcePush`
  (params (ActionValue :type Boolean) (ElapsedSeconds :type "Float (double-precision)") (TriggeredSeconds :type "Float (double-precision)") (InputAction :type "InputAction Object Reference" :default "/Game/Inputs/Actions/IA_ForcePush.IA_ForcePush"))
  (:`Triggered`
    (`MovementComponent.StopMovementImmediately` (`self.CharacterMovement`))
    (set `self.CanMove` false)
    (`self.PlayAnimMontage` "/Game/Player/Animations/Push_Montage.Push_Montage")
    (`KismetSystemLibrary.Delay` 0.45)
    (set `self.CanMove` true)
    (bind _hitactor (`self.TraceForPushables` "ForDuration")
      (:`HitPushable`
        (message `/Game/Blueprints/Interfaces/BPI_Pushable.OnPushed` _hitactor self)))))

(fn `GetForwardReachPoint`
  (params (StartingComponenet :type "SceneComponent Object Reference"))
  (returns (ReturnValue :type "Vector Structure"))
  (return (+ (`SceneComponent.K2_GetComponentLocation` StartingComponenet) (* (`SceneComponent.GetForwardVector` StartingComponenet) (`self.PushRange`)))))

(fn `UserConstructionScript`)